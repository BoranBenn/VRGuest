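; BP_Wood is a physics wood piece that can be grabbed by a hand, thrown, dropped or shattered.
; An integer WoodState tracks resting, held, airborne and shattered; airborne pieces are targetable and can optionally damage BP_RunningEnemy on hit.
; Tick returns airborne wood to rest once physics sleeps or it stays slow on walkable ground for a set time.
; Shatter spawns fragments, plays sound, reports AI noise and destroys the actor.
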(event `self.ReceiveTick`
  (params (DeltaSeconds :type "Float (single-precision)"))
  (`self.UpdateRestDetection` DeltaSeconds))

(event `self.ReceiveHit`
  (params (MyComp :type "PrimitiveComponent Object Reference") (Other :type "Actor Object Reference") (OtherComp :type "PrimitiveComponent Object Reference") (bSelfMoved :type Boolean) (HitLocation :type "Vector Structure") (HitNormal :type "Vector Structure") (NormalImpulse :type "Vector Structure") (Hit :type "HitResult Structure (by ref)"))
  (bind _bairborne (`self.IsAirborne`))
  (if (and (`self.bA2_WoodHitKillsEnemy`) _bairborne)
    (bind _asbp_running_enemy (cast `/Game/Enemies/BP_RunningEnemy` Other))
    (`GameplayStatics.ApplyDamage` _asbp_running_enemy 1.0 null self)))

(fn `ChangeWoodState`
  (params (NewState :type Integer))
  (set `self.WoodState` NewState)
  (set `self.RestAccum` 0.0))

(fn `DistanceToPoint`
  (params (Point :type "Vector Structure"))
  (returns (Distance :type "Float (double-precision)"))
  (return (`.ReturnValue` (`PrimitiveComponent.GetClosestPointOnCollision` (`self.Mesh`) Point "None"))))

(fn `IsAirborne`
  (returns (bAirborne :type Boolean))
  (bind _woodstate (`self.WoodState`))
  (return (or (== _woodstate 2) (== _woodstate 3))))

(fn `IsTargetable`
  (returns (bTargetable :type Boolean))
  (bind _woodstate (`self.WoodState`))
  (return (or (== _woodstate 2) (== _woodstate 3))))

(fn `OnGrabbed`
  (params (Hand :type "SceneComponent Object Reference"))
  (`PrimitiveComponent.SetSimulatePhysics` (`self.Mesh`) false)
  (`self.K2_AttachToComponent` self Hand "None" "KeepWorld" "KeepWorld" "KeepWorld" false)
  (set `self.HoldingHand` Hand)
  (set `self.bThrownByPlayer` false)
  (`self.ChangeWoodState` 1))

(fn `Shatter`
  (bind _returnvalue (`self.K2_GetActorLocation`))
  (`self.ChangeWoodState` 4)
  (for _ (range (+ (- (`self.FragmentCount`) 1) 1))
    (`|SpawnActorFromClass` "/Game/Wood/BP_WoodFragment.BP_WoodFragment_C" (`KismetMathLibrary.MakeTransform` (+ _returnvalue (* (`KismetMathLibrary.RandomUnitVector`) 10.0)) (`self.K2_GetActorRotation`)) "AlwaysSpawn" "MultiplyWithRoot" null null))
  (`GameplayStatics.PlaySoundAtLocation` (`self.BreakSound`) _returnvalue (struct) 1.0 1.0 0.0 null null null null)
  (`AISense_Hearing.ReportNoiseEvent` _returnvalue (`self.BreakNoiseLoudness`) (`GameplayStatics.GetPlayerPawn` 0) (`self.BreakNoiseRange`) "WoodBreak")
  (`self.K2_DestroyActor` self))

(fn `StartDropped`
  (`PrimitiveComponent.SetSimulatePhysics` (`self.Mesh`) true)
  (set `self.bThrownByPlayer` false)
  (`self.ChangeWoodState` 3))

(fn `Throw`
  (params (LinearVelocity :type "Vector Structure") (AngularVelocityDeg :type "Vector Structure") (bByPlayer :type Boolean))
  (bind _mesh (`self.Mesh`))
  (`self.K2_DetachFromActor` self "KeepWorld" "KeepWorld" "KeepWorld")
  (`PrimitiveComponent.SetSimulatePhysics` _mesh true)
  (`PrimitiveComponent.SetPhysicsLinearVelocity` _mesh (* LinearVelocity (`self.ThrowSpeedMultiplier`)) false "None")
  (`PrimitiveComponent.SetPhysicsAngularVelocityInDegrees` _mesh AngularVelocityDeg false "None")
  (set `self.HoldingHand` null)
  (set `self.bThrownByPlayer` bByPlayer)
  (if bByPlayer
    (`self.ChangeWoodState` 2)
    (else
      (`self.ChangeWoodState` 3))))

(fn `UpdateRestDetection`
  (params (DeltaSeconds :type "Float (double-precision)"))
  (bind _mesh (`self.Mesh`))
  (bind (_origin _boxextent) (`KismetSystemLibrary.GetComponentBounds` _mesh))
  (bind _bairborne (`self.IsAirborne`))
  (if _bairborne
    (bind _returnvalue (`PrimitiveComponent.GetPhysicsLinearVelocity` _mesh "None"))
    (bind (_outhit _returnvalue_2) (`KismetSystemLibrary.LineTraceSingle` _origin (- _origin (`KismetMathLibrary.MakeVector` 0.0 0.0 (+ (.z _boxextent) (`self.RestProbeDistance`)))) "TraceTypeQuery1" false (`|MakeArray` self)))
    (if (or (not (`PrimitiveComponent.IsAnyRigidBodyAwake` _mesh)) (and (and _returnvalue_2 (>= (.z (`.Normal` (`GameplayStatics.BreakHitResult` _outhit))) (`self.WalkableNormalZ`))) (< (`KismetMathLibrary.VSize` _returnvalue) (`self.RestSpeed`))))
      (set `self.RestAccum` (+ (`self.RestAccum`) DeltaSeconds))
      (else
        (set `self.RestAccum` 0.0)))
    (if (>= (`self.RestAccum`) (`self.RestTime`))
      (`self.ChangeWoodState` 0))))

(fn `UserConstructionScript`)