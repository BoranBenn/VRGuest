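; BP_WoodFragment is a short-lived physics debris piece of wood that flies off in a random direction when spawned.
; On BeginPlay it sets its lifespan and makes its mesh ignore the Pawn, Visibility and Camera channels, so it does not block characters, traces or the camera.
; It then gives the mesh a random linear velocity scaled by Speed and a random fixed-rate spin.
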(event `self.ReceiveBeginPlay`
  (bind _mesh (`self.Mesh`))
  (`self.SetLifeSpan` self (`self.Lifetime`))
  (`PrimitiveComponent.SetCollisionResponseToChannel` _mesh "ECC_Pawn" "ECR_Ignore")
  (`PrimitiveComponent.SetCollisionResponseToChannel` _mesh "ECC_Visibility" "ECR_Ignore")
  (`PrimitiveComponent.SetCollisionResponseToChannel` _mesh "ECC_Camera" "ECR_Ignore")
  (`PrimitiveComponent.SetPhysicsLinearVelocity` _mesh (* (`KismetMathLibrary.RandomUnitVector`) (`self.Speed`)) false "None")
  (`PrimitiveComponent.SetPhysicsAngularVelocityInDegrees` _mesh (* (`KismetMathLibrary.RandomUnitVector`) 720.0) false "None"))

(fn `UserConstructionScript`)