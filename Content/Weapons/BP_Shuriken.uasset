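; Thrown shuriken weapon that damages running enemies on impact.
; On BeginPlay its mesh takes the PhysicsActor profile with collision disabled; nothing here launches it or starts physics.
; Hits count only while the mesh simulates physics: BP_RunningEnemy takes damage and BP_Wood is ignored.
; Any other hit stops physics and switches the mesh to query-only collision, leaving the shuriken fixed in place.
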(event `self.ReceiveBeginPlay`
  (`PrimitiveComponent.SetCollisionProfileName` (`self.Mesh`) "PhysicsActor" true)
  (`PrimitiveComponent.SetCollisionEnabled` (`self.Mesh`) "NoCollision"))

(event `self.ReceiveHit`
  (params (MyComp :type "PrimitiveComponent Object Reference") (Other :type "Actor Object Reference") (OtherComp :type "PrimitiveComponent Object Reference") (bSelfMoved :type Boolean) (HitLocation :type "Vector Structure") (HitNormal :type "Vector Structure") (NormalImpulse :type "Vector Structure") (Hit :type "HitResult Structure (by ref)"))
  (bind _mesh (`self.Mesh`))
  (if (`SceneComponent.IsSimulatingPhysics` _mesh "None")
    (bind _asbp_running_enemy (cast `/Game/Enemies/BP_RunningEnemy` Other)
      (:`then`
        (`GameplayStatics.ApplyDamage` _asbp_running_enemy 1.0 null self))
      (:`CastFailed`
        (cast `/Game/Wood/BP_Wood` Other
          (:`CastFailed`
            (`PrimitiveComponent.SetSimulatePhysics` _mesh false)
            (`PrimitiveComponent.SetCollisionEnabled` _mesh "QueryOnly")))))))

(fn `UserConstructionScript`)