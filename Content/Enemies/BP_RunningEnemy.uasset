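; BP_RunningEnemy is a melee enemy that chases the player and is destroyed by any damage.
; Tick measures horizontal distance to the player camera, attacking within range or otherwise chasing beyond a stop distance.
; UpdatePath throttles AI MoveTo requests, with direct movement input as fallback when pathing fails.
; Attack plays a montage, then after a delay rechecks range with slack before damaging the player, skipping pawns tagged Reacquiring.
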(event `self.ReceiveTick`
  (params (DeltaSeconds :type "Float (single-precision)"))
  (bind _returnvalue (`GameplayStatics.GetPlayerCameraManager` 0))
  (bind _returnvalue_2 (- (`PlayerCameraManager.GetCameraLocation` _returnvalue) (`self.K2_GetActorLocation`)))
  (bind _returnvalue_3 (`KismetMathLibrary.MakeVector` (.x _returnvalue_2) (.y _returnvalue_2)))
  (bind _returnvalue_4 (`KismetMathLibrary.VSize` _returnvalue_3))
  (if (not (or (`self.bIsDead`) (`self.bIsAttacking`)))
    (`/Engine/EditorBlueprintResources/StandardMacros.IsValid` _returnvalue
      (:`Is Valid`
        (if (<= _returnvalue_4 (`self.AttackRange`))
          (`Controller.StopMovement` (`self.GetController`))
          (`self.Attack`)
          (elif (> _returnvalue_4 (`self.StopDistance`))
            (`self.UpdatePath`)
            (if (`self.bNavFailed`)
              (`self.AddMovementInput` (`KismetMathLibrary.Normal` _returnvalue_3)))))))))

(event `self.ReceiveAnyDamage`
  (params (Damage :type "Float (single-precision)") (DamageType :type "DamageType Object Reference") (InstigatedBy :type "Controller Object Reference") (DamageCauser :type "Actor Object Reference"))
  (set `self.bIsDead` true)
  (`self.K2_DestroyActor`))

(event `Attack`
  (set `self.bIsAttacking` true)
  (`AnimInstance.PlaySlotAnimationAsDynamicMontage` (`SkeletalMeshComponent.GetAnimInstance` (`self.Mesh`)) "/Game/Characters/Mannequins/Anims/Unarmed/Attack/MM_Attack_01.MM_Attack_01" "DefaultSlot" 0.1 0.2 1.0 1 -1.0 0.0)
  (`KismetSystemLibrary.Delay` (`self.HitDelay`))
  (`self.TryHitPlayer_0`)
  (`KismetSystemLibrary.Delay` (`self.AttackCooldown`))
  (set `self.bIsAttacking` false))

(fn `TryHitPlayer_0`
  (bind _returnvalue (`GameplayStatics.GetPlayerCameraManager` 0))
  (bind _returnvalue_2 (- (`PlayerCameraManager.GetCameraLocation` _returnvalue) (`self.K2_GetActorLocation`)))
  (if (not (or (`self.bIsDead`) (`self.ActorHasTag` (`GameplayStatics.GetPlayerPawn` 0) "Reacquiring")))
    (`/Engine/EditorBlueprintResources/StandardMacros.IsValid` _returnvalue
      (:`Is Valid`
        (if (<= (`KismetMathLibrary.VSize` (`KismetMathLibrary.MakeVector` (.x _returnvalue_2) (.y _returnvalue_2))) (+ (`self.AttackRange`) 40.0))
          (`GameplayStatics.ApplyDamage` (`GameplayStatics.GetPlayerPawn` 0) 1.0 (`self.GetController`) self))))))

(fn `UpdatePath`
  (bind _returnvalue (`GameplayStatics.GetRealTimeSeconds`))
  (bind _returnvalue_2 (`PlayerCameraManager.GetCameraLocation` (`GameplayStatics.GetPlayerCameraManager` 0)))
  (if (>= _returnvalue (`self.NextRepathTime`))
    (set `self.NextRepathTime` (+ _returnvalue (`self.RepathInterval`)))
    (bind _asaicontroller (cast `AIController` (`self.GetController`))
      (:`then`
        (bind _returnvalue_3 (`AIController.MoveToLocation` _asaicontroller (`KismetMathLibrary.MakeVector` (.x _returnvalue_2) (.y _returnvalue_2) (.z (`self.K2_GetActorLocation`))) (`self.StopDistance`) false true true false null true))
        (switch `EPathFollowingRequestResult` _returnvalue_3
          (:`Failed`
            (set `self.bNavFailed` true))
          (:`AlreadyAtGoal`
            (set `self.bNavFailed` false))
          (:`RequestSuccessful`
            (set `self.bNavFailed` false))))
      (:`CastFailed`
        (set `self.bNavFailed` true)))))

(fn `UserConstructionScript`)