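; Ranged enemy that turns in place to face the player's camera and shoots BP_EnemyBullet from a hand-socketed gun.
; Tick updates stun, then, while alive, yaws at constant speed and calls Fire once aim is within tolerance and the cooldown has elapsed.
; Turning and firing pause while the player pawn is tagged "Reacquiring".
; Fire spawns bullets slightly ahead of the gun, aimed just below the camera.
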(event `self.ReceiveBeginPlay`
  (set `self.NextFireTime` (+ (`KismetSystemLibrary.GetGameTimeInSeconds`) (`self.FirstShotDelay`)))
  (`SceneComponent.K2_AttachToComponent` (`self.Gun`) (`self.Mesh`) "HandGrip_R" "SnapToTarget" "SnapToTarget" "KeepWorld" false))

(event `self.ReceiveActorBeginOverlap`
  (params (OtherActor :type "Actor Object Reference"))
  (`parent.ReceiveActorBeginOverlap` OtherActor))

(event `self.ReceiveTick`
  (params (DeltaSeconds :type "Float (single-precision)"))
  (bind _returnvalue (`GameplayStatics.GetPlayerCameraManager` 0))
  (bind _yaw (.yaw (`KismetMathLibrary.FindLookAtRotation` (`self.K2_GetActorLocation`) (`PlayerCameraManager.GetCameraLocation` _returnvalue))))
  (`self.UpdateStun`)
  (if (not (`self.bIsDead`))
    (`/Engine/EditorBlueprintResources/StandardMacros.IsValid` _returnvalue
      (:`Is Valid`
        (if (not (`self.ActorHasTag` (`GameplayStatics.GetPlayerPawn` 0) "Reacquiring"))
          (`self.K2_SetActorRotation` (`KismetMathLibrary.RInterpTo_Constant` (`self.K2_GetActorRotation`) (`KismetMathLibrary.MakeRotator` 0.0 0.0 _yaw) DeltaSeconds (`self.TurnSpeed`)))
          (if (and (>= (`KismetSystemLibrary.GetGameTimeInSeconds`) (`self.NextFireTime`)) (< (`KismetMathLibrary.Abs` (`KismetMathLibrary.NormalizeAxis` (- _yaw (.yaw (`self.K2_GetActorRotation`))))) (`self.AimTolerance`)))
            (`self.Fire`)))))))

(fn `Fire`
  (bind _returnvalue (`SceneComponent.K2_GetComponentLocation` (`self.Gun`)))
  (bind _returnvalue_2 (- (`PlayerCameraManager.GetCameraLocation` (`GameplayStatics.GetPlayerCameraManager` 0)) (`KismetMathLibrary.MakeVector` 0.0 0.0 25.0)))
  (bind _returnvalue_3 (+ _returnvalue (* (`KismetMathLibrary.Normal` (- _returnvalue_2 _returnvalue)) 25.0)))
  (set `self.NextFireTime` (+ (`KismetSystemLibrary.GetGameTimeInSeconds`) (`self.FireInterval`)))
  (`|SpawnActorFromClass` "/Game/Enemies/BP_EnemyBullet.BP_EnemyBullet_C" (`KismetMathLibrary.MakeTransform` _returnvalue_3 (`KismetMathLibrary.FindLookAtRotation` _returnvalue_3 _returnvalue_2)) "AlwaysSpawn" "MultiplyWithRoot" self null))

(fn `UserConstructionScript`
  (`parent.UserConstructionScript`))