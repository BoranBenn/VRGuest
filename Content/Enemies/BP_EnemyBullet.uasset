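; BP_EnemyBullet is an enemy projectile that damages the player on a near pass and destroys itself.
; Each Tick it measures its distance to a vertical segment running from just above the player camera down past it, a capsule-like body test that avoids collision overlaps.
; Coming within the radius applies damage to the player pawn and destroys the bullet.
; Any Hit event also destroys it, without applying damage.
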(event `self.ReceiveTick`
  (params (DeltaSeconds :type "Float (single-precision)"))
  (bind _returnvalue (`GameplayStatics.GetPlayerCameraManager` 0))
  (bind _returnvalue_2 (`PlayerCameraManager.GetCameraLocation` _returnvalue))
  (`/Engine/EditorBlueprintResources/StandardMacros.IsValid` _returnvalue
    (:`Is Valid`
      (if (< (`KismetMathLibrary.GetPointDistanceToSegment` (`self.K2_GetActorLocation`) (+ _returnvalue_2 (`KismetMathLibrary.MakeVector` 0.0 0.0 10.0)) (- _returnvalue_2 (`KismetMathLibrary.MakeVector` 0.0 0.0 130.0))) 22.0)
        (`GameplayStatics.ApplyDamage` (`GameplayStatics.GetPlayerPawn` 0) 1.0 null self)
        (`self.K2_DestroyActor`)))))

(event `self.ReceiveHit`
  (params (MyComp :type "PrimitiveComponent Object Reference") (Other :type "Actor Object Reference") (OtherComp :type "PrimitiveComponent Object Reference") (bSelfMoved :type Boolean) (HitLocation :type "Vector Structure") (HitNormal :type "Vector Structure") (NormalImpulse :type "Vector Structure") (Hit :type "HitResult Structure (by ref)"))
  (`self.K2_DestroyActor`))

(fn `UserConstructionScript`)