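; Sniper enemy that punishes players who camp on high ground.
; Each tick it updates stun and, while alive, yaws toward the player camera at a limited speed.
; A player above a height threshold, within aim tolerance of an unstunned sniper, starts a grace timer, then a timed aim, firing and cooldown.
; A scaled beam mesh telegraphs the shot by changing thickness, and the "Reacquiring" player tag resets everything.
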(event `self.ReceiveTick`
  (params (DeltaSeconds :type "Float (single-precision)"))
  (`self.UpdateStun`)
  (if (`self.bIsDead`)
    (`self.UpdateAimBeam` false)
    (else
      (`self.SniperTick`))))

(fn `SniperTick`
  (bind _returnvalue (`KismetSystemLibrary.GetGameTimeInSeconds`))
  (bind _returnvalue_2 (`PlayerCameraManager.GetCameraLocation` (`GameplayStatics.GetPlayerCameraManager` 0)))
  (bind _returnvalue_3 (- _returnvalue_2 (`KismetMathLibrary.MakeVector` 0.0 0.0 25.0)))
  (bind _yaw (.yaw (`KismetMathLibrary.FindLookAtRotation` (`self.K2_GetActorLocation`) _returnvalue_2)))
  (if (`self.ActorHasTag` (`GameplayStatics.GetPlayerPawn` 0) "Reacquiring")
    (set `self.HighSince` -1.0)
    (set `self.AimStart` -1.0)
    (`self.UpdateAimBeam` false _returnvalue_3)
    (else
      (`self.K2_SetActorRotation` (`KismetMathLibrary.RInterpTo_Constant` (`self.K2_GetActorRotation`) (`KismetMathLibrary.MakeRotator` 0.0 0.0 _yaw) (`GameplayStatics.GetWorldDeltaSeconds`) (`self.TurnSpeed`)))
      (if (and (> (.z (`self.K2_GetActorLocation` (`GameplayStatics.GetPlayerPawn` 0))) (`self.HighGroundMinZ`)) (and (< (`KismetMathLibrary.Abs` (`KismetMathLibrary.NormalizeAxis` (- _yaw (.yaw (`self.K2_GetActorRotation`))))) (`self.AimTolerance`)) (not (`self.bStunned`))))
        (if (< (`self.HighSince`) 0.0)
          (set `self.HighSince` _returnvalue))
        (if (>= (- _returnvalue (`self.HighSince`)) (`self.CampGraceTime`))
          (if (< (`self.AimStart`) 0.0)
            (set `self.AimStart` _returnvalue))
          (if (>= (- _returnvalue (`self.AimStart`)) (`self.AimTime`))
            (`self.Fire`)
            (set `self.AimStart` -1.0)
            (set `self.HighSince` (- (+ _returnvalue (`self.SniperCooldown`)) (`self.CampGraceTime`)))
            (`self.UpdateAimBeam` false _returnvalue_3)
            (else
              (`self.UpdateAimBeam` true _returnvalue_3)))
          (else
            (`self.UpdateAimBeam` false _returnvalue_3)))
        (else
          (set `self.HighSince` -1.0)
          (set `self.AimStart` -1.0)
          (`self.UpdateAimBeam` false _returnvalue_3))))))

(fn `UpdateAimBeam`
  (params (bShow :type Boolean) (Target :type "Vector Structure"))
  (bind _aimbeam (`self.AimBeam`))
  (bind _returnvalue (`SceneComponent.K2_GetComponentLocation` (`self.Gun`)))
  (bind _returnvalue_2 (- Target _returnvalue))
  (bind _returnvalue_3 (/ (- (`KismetSystemLibrary.GetGameTimeInSeconds`) (`self.AimStart`)) (`self.AimTime`)))
  (bind _returnvalue_4 (`KismetMathLibrary.Lerp` (`self.BeamThicknessStart`) (`self.BeamThicknessEnd`) (select `bool` (> _returnvalue_3 1.0) :`false` _returnvalue_3 :`true` 1.0)))
  (`SceneComponent.SetVisibility` _aimbeam bShow false)
  (if bShow
    (`SceneComponent.K2_SetWorldLocationAndRotation` _aimbeam (* (+ _returnvalue Target) 0.5) (`KismetMathLibrary.MakeRotFromZ` _returnvalue_2) false false)
    (`SceneComponent.SetWorldScale3D` _aimbeam (`KismetMathLibrary.MakeVector` (/ _returnvalue_4 100.0) (/ _returnvalue_4 100.0) (/ (`KismetMathLibrary.VSize` _returnvalue_2) 100.0)))))

(fn `UserConstructionScript`
  (`parent.UserConstructionScript`))