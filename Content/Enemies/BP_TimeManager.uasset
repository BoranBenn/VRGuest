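; BP_TimeManager links global time dilation to how fast the player's camera turns, slowing the game while the view is still.
; Each Tick converts angular change in camera forward into an undilated turn rate, maps it between minimum scale and normal speed, then smooths it.
; BP_XRPawn death, aiming or swapping suspends this control, with swapping forcing normal speed.
; EndPlay restores normal time.
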(event `self.ReceiveTick`
  (params (DeltaSeconds :type "Float (single-precision)"))
  (bind _returnvalue (`GameplayStatics.GetPlayerCameraManager` 0))
  (bind _lastforward (`self.LastForward`))
  (bind _returnvalue_2 (/ DeltaSeconds (`GameplayStatics.GetGlobalTimeDilation`)))
  (bind _returnvalue_3 (`KismetMathLibrary.GetForwardVector` (`PlayerCameraManager.GetCameraRotation` _returnvalue)))
  (`self.HandlePlayerTimeOverride`)
  (if (not (`self.bPlayerOverride`))
    (`/Engine/EditorBlueprintResources/StandardMacros.IsValid` _returnvalue
      (:`Is Valid`
        (set `self.CurrentTimeScale` (`KismetMathLibrary.FInterpTo` (`self.CurrentTimeScale`) (`KismetMathLibrary.MapRangeClamped` (/ (select `bool` (> (`KismetMathLibrary.VSize` _lastforward) 0.5) :`false` 0.0 :`true` (`KismetMathLibrary.DegAcos` (`KismetMathLibrary.FClamp` (`KismetMathLibrary.Dot_VectorVector` _returnvalue_3 _lastforward) -1.0))) (`KismetMathLibrary.FMax` _returnvalue_2 0.0001)) 0.0 (`self.FullSpeedTurnRate`) (`self.MinTimeScale`) 1.0) _returnvalue_2 (`self.SmoothSpeed`)))
        (`GameplayStatics.SetGlobalTimeDilation` (`self.CurrentTimeScale`))
        (set `self.LastForward` _returnvalue_3)))))

(event `self.ReceiveEndPlay`
  (params (EndPlayReason :type "EEndPlayReason Enum" :default "Destroyed"))
  (`GameplayStatics.SetGlobalTimeDilation` 1.0))

(fn `HandlePlayerTimeOverride`
  (bind _returnvalue (`GameplayStatics.GetPlayerCameraManager` 0))
  (set `self.bPlayerOverride` false)
  (bind _asbp_xrpawn (cast `/Game/XRFramework/Blueprints/BP_XRPawn` (`GameplayStatics.GetPlayerPawn` 0)))
  (if (`/Game/XRFramework/Blueprints/BP_XRPawn.PlayerDead` _asbp_xrpawn)
    (set `self.bPlayerOverride` true)
    (else
      (bind _isswapping (`/Game/XRFramework/Blueprints/BP_XRPawn.IsSwapping` _asbp_xrpawn))
      (if (or (`/Game/XRFramework/Blueprints/BP_XRPawn.isAiming` _asbp_xrpawn) _isswapping)
        (set `self.bPlayerOverride` true)
        (`/Engine/EditorBlueprintResources/StandardMacros.IsValid` _returnvalue
          (:`Is Valid`
            (set `self.LastForward` (`KismetMathLibrary.GetForwardVector` (`PlayerCameraManager.GetCameraRotation` _returnvalue)))
            (if _isswapping
              (set `self.CurrentTimeScale` 1.0)
              (`GameplayStatics.SetGlobalTimeDilation` 1.0))))))))

(fn `UserConstructionScript`)