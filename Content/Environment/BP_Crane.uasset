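; Crane actor that shuttles a trolley back and forth while periodically dropping BP_Wood pallets into the level.
; BeginPlay sizes the rope and hook; while CraneActive, Tick moves the hoist between its travel limits and runs the pallet cycle.
; Pallets spawn attached to LoadPoint after a reload delay, capped by the level's BP_Wood count.
; Timed drops wait until LoadPoint clears the padded XY bounds of ForbiddenTag actors.
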(event `self.ReceiveBeginPlay`
  (`self.ApplyRope`))

(event `self.ReceiveTick`
  (params (DeltaSeconds :type "Float (single-precision)"))
  (if (`self.bCraneActive`)
    (`self.UpdateTrolley`)
    (`self.UpdatePallet`)))

(fn `ApplyRope`
  (bind _ropelength (`self.RopeLength`))
  (`SceneComponent.SetRelativeScale3D` (`self.Rope`) (`KismetMathLibrary.MakeVector` 1.0 1.0 (/ _ropelength 100.0)))
  (`SceneComponent.K2_SetRelativeLocation` (`self.Hook`) (`KismetMathLibrary.MakeVector` 0.0 0.0 (- -77.9 _ropelength)) false false))

(fn `CanDropHere`
  (returns (Allowed :type Boolean))
  (bind _returnvalue (`SceneComponent.K2_GetComponentLocation` (`self.LoadPoint`)))
  (bind _outactors (`GameplayStatics.GetAllActorsWithTag` (`self.ForbiddenTag`)))
  (for _array_element _outactors
    (bind (_origin _boxextent) (`self.GetActorBounds` _array_element true false))
    (if (and (< (`KismetMathLibrary.Abs` (- (.x _returnvalue) (.x _origin))) (+ (.x _boxextent) 70.0)) (< (`KismetMathLibrary.Abs` (- (.y _returnvalue) (.y _origin))) (+ (.y _boxextent) 70.0)))
      (return (not true))))
  (return (not false)))

(fn `DropPallet`
  (bind _heldpallet (`self.HeldPallet`))
  (`self.K2_DetachFromActor` _heldpallet "KeepWorld" "KeepWorld" "KeepWorld")
  (`/Game/Wood/BP_Wood.StartDropped` _heldpallet)
  (set `self.HeldPallet` null)
  (set `self.NextReloadTime` (+ (`KismetSystemLibrary.GetGameTimeInSeconds`) (`self.ReloadTime`))))

(fn `IsDropAllowed_0`
  (returns (Allowed :type Boolean)))

(fn `SpawnPallet`
  (bind _loadpoint (`self.LoadPoint`))
  (bind _returnvalue (`|SpawnActorFromClass` "/Game/Wood/BP_Wood.BP_Wood_C" (`SceneComponent.K2_GetComponentToWorld` _loadpoint) "AlwaysSpawn" "MultiplyWithRoot" null null))
  (bind _asstatic_mesh_component (cast `StaticMeshComponent` (`self.GetComponentByClass` _returnvalue "/Script/Engine.StaticMeshComponent")))
  (`PrimitiveComponent.SetSimulatePhysics` _asstatic_mesh_component false)
  (`StaticMeshComponent.SetStaticMesh` _asstatic_mesh_component (`self.PalletMesh`))
  (`PrimitiveComponent.SetMaterial` _asstatic_mesh_component 0 (`self.PalletMaterial`))
  (`self.SetActorScale3D` _returnvalue (`KismetMathLibrary.MakeVector` 1.0 1.0 1.0))
  (`self.K2_AttachToComponent` _returnvalue _loadpoint "None" "SnapToTarget" "SnapToTarget" "KeepWorld" true)
  (`/Game/Wood/BP_Wood.ChangeWoodState` _returnvalue 1)
  (set `self.HeldPallet` _returnvalue)
  (set `self.NextDropTime` (+ (`KismetSystemLibrary.GetGameTimeInSeconds`) (`self.DropInterval`))))

(fn `UpdatePallet`
  (bind _returnvalue (`KismetSystemLibrary.GetGameTimeInSeconds`))
  (`/Engine/EditorBlueprintResources/StandardMacros.IsValid` (`self.HeldPallet`)
    (:`Is Valid`
      (bind _allowed (`self.CanDropHere`))
      (if (and _allowed (>= _returnvalue (`self.NextDropTime`)))
        (`self.DropPallet`)))
    (:`Is Not Valid`
      (bind _outactors (`GameplayStatics.GetAllActorsOfClass` "/Game/Wood/BP_Wood.BP_Wood_C"))
      (if (and (>= _returnvalue (`self.NextReloadTime`)) (< (`KismetArrayLibrary.Array_Length` _outactors) (`self.MaxWoodInLevel`)))
        (`self.SpawnPallet`)))))

(fn `UpdateTrolley`
  (bind _traveldir (`self.TravelDir`))
  (bind _travelextent (`self.TravelExtent`))
  (bind _returnvalue (+ (`self.TrolleyX`) (* (* _traveldir (`self.TravelSpeed`)) (`GameplayStatics.GetWorldDeltaSeconds`))))
  (if (> (`KismetMathLibrary.Abs` _returnvalue) _travelextent)
    (set `self.TravelDir` (- 0.0 _traveldir))
    (set `self.TrolleyX` (select `bool` (> _returnvalue 0.0) :`false` (- 0.0 _travelextent) :`true` _travelextent))
    (else
      (set `self.TrolleyX` _returnvalue)))
  (`SceneComponent.K2_SetRelativeLocation` (`self.Hoist`) (`KismetMathLibrary.MakeVector` (`self.TrolleyX`)) false false))

(fn `UserConstructionScript`)