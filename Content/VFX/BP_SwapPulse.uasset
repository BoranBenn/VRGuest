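; BP_SwapPulse is a short-lived VFX actor that plays an expanding, fading pulse on its static mesh and then destroys itself.
; BeginPlay creates a dynamic material instance and records the real-time spawn moment.
; Tick uses clamped elapsed real time over Duration to grow X and Y scale with a quadratic ease-out while linearly lowering the material's Fade parameter.
; Using real time keeps the pulse independent of time dilation.
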(event `self.ReceiveBeginPlay`
  (bind _returnvalue (`PrimitiveComponent.CreateDynamicMaterialInstance` (`self.StaticMeshComponent`) 0 null "None"))
  (set `self.PulseMID` _returnvalue)
  (set `self.SpawnRealTime` (`GameplayStatics.GetRealTimeSeconds`))
  (`self.SetActorScale3D` (`KismetMathLibrary.MakeVector` (`self.StartScale`) (`self.StartScale`) 1.0)))

(event `self.ReceiveTick`
  (params (DeltaSeconds :type "Float (single-precision)"))
  (bind _pulsemid (`self.PulseMID`))
  (bind _returnvalue (`KismetMathLibrary.FClamp` (/ (- (`GameplayStatics.GetRealTimeSeconds`) (`self.SpawnRealTime`)) (`KismetMathLibrary.FMax` (`self.Duration`) 0.01))))
  (bind _returnvalue_2 (- 1.0 _returnvalue))
  (bind _returnvalue_3 (`KismetMathLibrary.Lerp` (`self.StartScale`) (`self.MaxScale`) (- 1.0 (* _returnvalue_2 _returnvalue_2))))
  (`self.SetActorScale3D` (`KismetMathLibrary.MakeVector` _returnvalue_3 _returnvalue_3 1.0))
  (`/Engine/EditorBlueprintResources/StandardMacros.IsValid` _pulsemid
    (:`Is Valid`
      (`MaterialInstanceDynamic.SetScalarParameterValue` _pulsemid "Fade" _returnvalue_2)
      (if (>= _returnvalue 1.0)
        (`self.K2_DestroyActor`)))
    (:`Is Not Valid`
      (if (>= _returnvalue 1.0)
        (`self.K2_DestroyActor`)))))

(fn `UserConstructionScript`)